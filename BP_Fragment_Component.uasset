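; Destructible fragment actor that loses health when hit by projectiles flagged to affect destructibles.
; Each hit applies environmental damage and plays a timeline-driven color flash on a dynamic material instance created at construction.
; At the first health threshold it swaps to an indexed damaged mesh.
; At the second it calls DestroyActor, then reads a DataTable row by fragment index to add physics-simulated debris mesh components.
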(event `self.StaticMesh.OnComponentHit`
  (params (HitComponent :type "PrimitiveComponent Object Reference") (OtherActor :type "Actor Object Reference") (OtherComp :type "PrimitiveComponent Object Reference") (NormalImpulse :type "Vector Structure") (Hit :type "HitResult Structure (by ref)"))
  (bind _datatable (break `DataTableRowHandle` (`self.RowHandleFragmentParts`)))
  ;[1 1 1] Get Projectile Hit Component and Damage
  (bind _asbp_master_projectile (cast `/Game/FirstPerson/Blueprints/BP_Master_Projectile` OtherActor))
  (if (`/Game/FirstPerson/Blueprints/BP_Master_Projectile.CanAffectDestructible` _asbp_master_projectile)
    (`|ExecutionSequence`
      (:`then_0`
        (bind _returnvalue (`GameplayStatics.ApplyDamage` (`.HitActor` (`GameplayStatics.BreakHitResult` Hit)) (`KismetMathLibrary.Conv_IntToDouble` (`/Game/FirstPerson/Blueprints/BP_Master_Projectile.Damage` _asbp_master_projectile)) null null "/Engine/EngineDamageTypes/DmgTypeBP_Environmental.DmgTypeBP_Environmental_C"))
        (set `self.HitDamage` _returnvalue)
        ;[1 1 1] First Damage Threshold
        (bind _output_get (set `self.Health` (- (`self.Health`) (`self.HitDamage`))))
        (set `self.HitDamage` 0.0)
        (`KismetSystemLibrary.PrintString` (`KismetStringLibrary.Conv_DoubleToString` _output_get))
        (if (<= _output_get (`self.FirstDamageThreshold`))
          ;[1 1 1] Second Damage Threshold
          (`AddComponent|NODE_AddStaticMeshComponent-0` :`RelativeTransform` (`self.GetTransform`))
          (`StaticMeshComponent.SetStaticMesh` (`self.StaticMesh`) (`|GetArrayItem` (`self.VisualFragment`) (`self.FragmentIndex`)))
          (if (<= (`self.Health`) (`self.SecondDamageThreshold`))
            ;[1 1 1] Fragments Parts Spawn
            (`self.K2_DestroyActor`)
            (bind _outrownames (`DataTableFunctionLibrary.GetDataTableRowNames` _datatable))
            (bind _returnvalue_2 (`|GetDataTableRow` _datatable (`|GetArrayItem` _outrownames (`self.FragmentIndex`)))
              (:`then`
                (bind _structout (setmembers `/Game/Data_Tables/S_Fragment_Parts` :`StructRef` _returnvalue_2))
                (for _array_element (break `/Game/Data_Tables/S_Fragment_Parts` _structout)
                  (bind _returnvalue_3 (`AddComponent|NODE_AddStaticMeshComponent-2` :`RelativeTransform` (`self.RelativePosition`)))
                  (`StaticMeshComponent.SetStaticMesh` _returnvalue_3 _array_element)
                  (`PrimitiveComponent.SetSimulatePhysics` _returnvalue_3 true)))))))
      (:`then_1`
        ;[1 1 1] Hit Damage Visual Effect
        (bind (_direction _colortrack) (`Timeline|Timeline` :!via `PlayFromStart`)
          (:`Update`
            (`MaterialInstanceDynamic.SetVectorParameterValue` (`self.Material`) "Color" _colortrack)))))))

(fn `UserConstructionScript`
  (bind _returnvalue (`PrimitiveComponent.CreateDynamicMaterialInstance` (`self.StaticMesh`) 0 "/Game/Materials/M_Structure.M_Structure" "None"))
  (set `self.Material` _returnvalue))